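; Dialogue manager Blueprint that shows a line from a Dialogue array each time DisplayNextLine fires.
; It creates a W_Dialogue widget on BeginPlay, then shows it for five seconds per line while incrementing Index.
; The line text goes only to PrintText, not into the widget.
; A non-negative Index displays only when ShouldRepetText is set, resetting to the first line; a negative Index prints without resetting.
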(event Custom|DisplayNextLine
  (bind _dialoguewidget (Variables|Default|GetDialogueWidget))
  (if (>= (Variables|Default|GetIndex) 0)
    (if (Variables|Default|GetShouldRepetText)
      (Variables|Default|SetIndex 0)
      (Development|PrintText (Utilities|Array|Get(acopy) (Variables|Default|GetDialogue) (Variables|Default|GetIndex)) true true "(R=1.000000,G=0.256129,B=0.046370,A=1.000000)" :!label _label)
      (Utilities|FlowControl|Sequence
        (:then_0
          (UserInterface|Viewport|AddtoViewport _dialoguewidget 0)
          (Utilities|FlowControl|Delay 5.0)
          (Widget|RemovefromParent _dialoguewidget))
        (:then_1
          (Math|Integer|IncrementInt (Variables|Default|GetIndex)))))
    (else
      (goto _label))))

(event EventBeginPlay
  (bind _returnvalue (UserInterface|CreateWidget "/Game/Widgets/W_Dialogue.W_Dialogue_C"))
  (Variables|Default|SetDialogueWidget _returnvalue))

(fn ConstructionScript)