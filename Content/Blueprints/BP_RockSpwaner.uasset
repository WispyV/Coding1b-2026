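; BP_RockSpwaner is a pickup item, a "rock planter" the player can carry and use to plant objects.
; Overlapping a BP_ThirdPersonCharacter stores it as Player and calls its TryToPickupitem, and the Pickup event snaps the item to that character's right-hand IK socket.
; PrimaryAction spawns a BP_Tree at the item's transform, despite its rock-planting message.
; Drop destroys the item instead of detaching it.
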(event Collision|EventActorBeginOverlap
  (params (OtherActor :type Actor%20Object%20Reference))
  (bind _asbp_third_person_character (Utilities|Casting|CastToBP_ThirdPersonCharacter OtherActor))
  (Variables|Default|SetPlayer _asbp_third_person_character)
  (Default|TrytoPickupitem _asbp_third_person_character self))

(event EventPickup
  (Development|PrintText "The rock planter is getting picked up.")
  (Transformation|AttachComponentToComponent (Variables|/Script/Engine.Character|GetMesh (Variables|Default|GetPlayer)) "ik_hand_rSocket" "SnapToTarget" "SnapToTarget" "KeepRelative" true))

(event EventPrimaryAction
  (Development|PrintText "Plant this rock")
  (Game|SpawnActorfromClass "/Game/Blueprints/BP_Tree.BP_Tree_C" (Transformation|GetActorTransform) "Undefined" "MultiplyWithRoot" 0 0))

(event EventDrop
  (Development|PrintText "Drop")
  (Actor|DestroyActor))

(fn ConstructionScript)