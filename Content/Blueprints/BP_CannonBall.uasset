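; Cannonball actor that removes itself a few seconds after spawning.
; A Lights event, not called within this Blueprint, creates a dynamic material instance on the Cube component.
; It then loops on a delay, setting the emissive color to a random entry from the Colors array until the actor is destroyed.
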(event Custom|Lights
  (bind _returnvalue (Rendering|Material|CreateDynamicMaterialInstance (Variables|Default|GetCube) 0 0 "None" :!class /Script/Engine.PrimitiveComponent))
  (Variables|Default|SetDynamicMat _returnvalue)
  (Rendering|Material|SetVectorParameterValue (Variables|Default|GetDynamicMat) "Emissive Color" (.OutItem (Utilities|Array|Random (Variables|Default|GetColors))) :!class /Script/Engine.MaterialInstanceDynamic :!label _label)
  (Utilities|FlowControl|Delay 1.0)
  (goto _label))

(event EventBeginPlay
  (Utilities|FlowControl|Delay 3.0)
  (Actor|DestroyActor))

(fn ConstructionScript)