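; BP_cowboyBean is a cowboy bean actor that grows in random steps after play begins.
; On BeginPlay, a looping DoN gate allows a random one to four growth steps, each preceded by a random delay of a few seconds.
; Each step calls GrowC, which adds a small random amount to the relative scale of the SMBeanCowboy01 component.
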(event Custom|GrowC
  (bind _sm_bean_cowboy_01 (Variables|Default|GetSM_Bean_Cowboy_01))
  (Transformation|SetRelativeScale3D _sm_bean_cowboy_01 (+ (Variables|/Script/Engine.SceneComponent|GetRelativeScale3D _sm_bean_cowboy_01) (Math|Random|RandomFloatinRange 0.2 0.4))))

(event EventBeginPlay
  (bind _counter (Utilities|FlowControl|DoN (Math|Random|RandomIntegerinRange 1 4) :!label _label)
    (:Exit
      (Utilities|FlowControl|Delay (Math|Random|RandomFloatinRange 3.0 5.0))
      (CallFunction|GrowC)
      (if (not (== _counter 0))
        (goto _label)))))

(fn ConstructionScript)