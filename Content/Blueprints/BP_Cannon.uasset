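; BP_Cannon is a cannon actor that automatically fires cannonballs on a repeating timer.
; BeginPlay starts an endless loop that waits one second, then calls the FireCannon event.
; FireCannon prints a debug message, spawns a BP_CannonBall at the SpawnPoint transform and launches its Cube component along the SpawnPoint's forward vector with a mass-independent AddForce.
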(event Custom|FireCannon
  (Development|PrintText "Cannon is firing!")
  (bind _returnvalue (Game|SpawnActorfromClass "/Game/Blueprints/BP_CannonBall.BP_CannonBall_C" (Transformation|GetWorldTransform (Variables|Default|GetSpawnPoint)) "Undefined" "MultiplyWithRoot" 0 0))
  (Physics|AddForce (Variables|/Game/Blueprints/BP_CannonBall.BP_CannonBall_C|GetCube _returnvalue) (* (Math|Vector|GetForwardVector (Variables|Default|GetSpawnPoint)) 1e+05) "None" true))

(event EventBeginPlay
  (Utilities|FlowControl|Delay 1.0 :!label _label)
  (CallFunction|FireCannon)
  (goto _label))

(event Collision|EventActorBeginOverlap
  (params (OtherActor :type Actor%20Object%20Reference)))

(event EventTick
  (params (DeltaSeconds :type Float%20%28single-precision%29)))

(fn ConstructionScript)